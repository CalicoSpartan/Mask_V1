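; BP_FPSGameState is an FPS game state Blueprint that owns the gameplay HUD and posts kill feed messages to it.
; On BeginPlay it creates a GameplayUI widget, stores it and adds it to the viewport.
; CallHUDUpdate triggers a custom event that builds a KillFeedEntry widget from the KillFeedMessage variable and appends it to the HUD's vertical box.
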(event `self.ReceiveBeginPlay`
  (bind _returnvalue (`|CreateWidget` "/Game/UI/GameplayUI.GameplayUI_C"))
  (bind _output_get (set `self.UI` _returnvalue))
  (`UserWidget.AddToViewport` _output_get 0))

(event `CustomEvent_0`
  (bind _returnvalue (`|CreateWidget` "/Game/UI/KillFeedEntry.KillFeedEntry_C" null (`KismetTextLibrary.Conv_StringToText` (`self.KillFeedMessage`))))
  (bind _output_get (set `self.Entry` _returnvalue))
  (`VerticalBox.AddChildToVerticalBox` (`/Game/UI/GameplayUI.VerticalBox_0` (stale `self.ReceiveBeginPlay` _output_get)) _output_get))

(event `self.CallHUDUpdate`
  (`self.CustomEvent_0`))

(fn `UserConstructionScript`)